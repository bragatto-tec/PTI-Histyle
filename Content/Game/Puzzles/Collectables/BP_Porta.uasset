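; BP_Porta is an interactable door that swings open and closed with a sound for each direction.
; Interact sets the DoorTrack timeline's play rate from TimeToOpenS, then calls OpenDoor or CloseDoor based on IsOpen.
; The timeline plays or reverses to interpolate the door's relative yaw, and IsOpen flips only when it finishes.
; Both sounds play at the world origin rather than at the door.
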(event Custom|Open%20Door
  (Audio|PlaySoundatLocation "/Game/Game/Puzzles/Collectables/431117__inspectorj__door-front-opening-a.431117__inspectorj__door-front-opening-a" "0, 0, 0" "0, 0, 0" 1.0 1.0 0.0 0 0 0 0)
  (bind _door_track (Timeline|Door%20Track Play)
    (:Update
      (Transformation|SetRelativeRotation (Variables|Default|GetDoor) (Math|Rotator|MakeRotator 0.0 0.0 (Math|Float|Lerp (Variables|Default|GetOpen%20Position%20) (Variables|Default|GetClose%20Position) _door_track)) false false))
    (:Finished
      (Variables|Default|SetIsOpen? (not (Variables|Default|GetIsOpen?))))))

(event Custom|Close%20Door
  (Audio|PlaySoundatLocation "/Game/Game/Puzzles/Collectables/431118__inspectorj__door-front-closing-a.431118__inspectorj__door-front-closing-a" "0, 0, 0" "0, 0, 0" 1.0 1.0 0.0 0 0 0 0)
  (bind _door_track (Timeline|Door%20Track Reverse)
    (:Update
      (Transformation|SetRelativeRotation (Variables|Default|GetDoor) (Math|Rotator|MakeRotator 0.0 0.0 (Math|Float|Lerp (Variables|Default|GetOpen%20Position%20) (Variables|Default|GetClose%20Position) _door_track)) false false))
    (:Finished
      (Variables|Default|SetIsOpen? (not (Variables|Default|GetIsOpen?))))))

(fn ConstructionScript)

(fn Interact
  (params (Interactor :type Character%20Object%20Reference))
  (bind _door_track (Variables|Default|GetDoor%20Track))
  (if (not (Variables|Default|GetIsOpen?))
    (Components|Timeline|SetPlayRate _door_track (/ 1.0 (Variables|Default|GetTime%20to%20Open%20%28s%29)))
    (CallFunction|OpenDoor)
    (else
      (Components|Timeline|SetPlayRate _door_track (/ 1.0 (Variables|Default|GetTime%20to%20Open%20%28s%29)))
      (CallFunction|CloseDoor)))
  (return false))