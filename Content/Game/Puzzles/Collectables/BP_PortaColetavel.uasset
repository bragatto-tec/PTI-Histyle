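; BP_PortaColetavel is an interactable hinged door from the collectables puzzle folder.
; A box overlap shows or hides an interact prompt widget for the player.
; Interact checks IsOpen and plays or reverses the DoorTrack timeline, scaled by TimeToOpenS, with opening or closing sounds played at world origin.
; The timeline lerps door yaw between OpenPosition and ClosePosition and toggles IsOpen when finished.
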(event OnComponentBeginOverlap(Box)
  (params (OverlappedComponent :type Primitive%20Component%20Object%20Reference) (OtherActor :type Actor%20Object%20Reference) (OtherComp :type Primitive%20Component%20Object%20Reference) (OtherBodyIndex :type Integer) (bFromSweep :type Boolean) (SweepResult :type Hit%20Result%20Structure%20%28by%20ref%29))
  (Utilities|FlowControl|Sequence
    (:then_0
      (if (== OtherActor (Game|GetPlayerCharacter 0))
        (UserInterface|Viewport|AddtoViewport (Variables|Default|GetInteract%20Prompt) 0)))))

(event OnComponentEndOverlap(Box)
  (params (OverlappedComponent :type Primitive%20Component%20Object%20Reference) (OtherActor :type Actor%20Object%20Reference) (OtherComp :type Primitive%20Component%20Object%20Reference) (OtherBodyIndex :type Integer))
  (Utilities|FlowControl|Sequence
    (:then_0
      (if (== (Game|GetPlayerCharacter 0) OtherActor)
        (Widget|RemovefromParent (Variables|Default|GetInteract%20Prompt))))))

(event Custom|Open%20Door
  (Audio|PlaySoundatLocation "/Game/Game/Puzzles/Collectables/431117__inspectorj__door-front-opening-a.431117__inspectorj__door-front-opening-a" "0, 0, 0" "0, 0, 0" 1.0 1.0 0.0 0 0 0 0)
  (bind _door_track (Timeline|Door%20Track Play)
    (:Update
      (Transformation|SetRelativeRotation (Variables|Default|GetDoor) (Math|Rotator|MakeRotator 0.0 0.0 (Math|Float|Lerp (Variables|Default|GetOpen%20Position%20) (Variables|Default|GetClose%20Position) _door_track)) false false))
    (:Finished
      (Variables|Default|SetIsOpen? (not (Variables|Default|GetIsOpen?))))))

(event Custom|Close%20Door
  (Audio|PlaySoundatLocation "/Game/Game/Puzzles/Collectables/431118__inspectorj__door-front-closing-a.431118__inspectorj__door-front-closing-a" "0, 0, 0" "0, 0, 0" 1.0 1.0 0.0 0 0 0 0)
  (bind _door_track (Timeline|Door%20Track Reverse)
    (:Update
      (Transformation|SetRelativeRotation (Variables|Default|GetDoor) (Math|Rotator|MakeRotator 0.0 0.0 (Math|Float|Lerp (Variables|Default|GetOpen%20Position%20) (Variables|Default|GetClose%20Position) _door_track)) false false))
    (:Finished
      (Variables|Default|SetIsOpen? (not (Variables|Default|GetIsOpen?))))))

(event EventBeginPlay
  (bind _returnvalue (UserInterface|CreateWidget "/Game/Game/Widgets/P_Interact.P_Interact_C"))
  (Variables|Default|SetInteract%20Prompt _returnvalue))

(fn ConstructionScript)

(fn Interact
  (params (Interactor :type Character%20Object%20Reference))
  (bind _door_track (Variables|Default|GetDoor%20Track))
  (if (not (Variables|Default|GetIsOpen?))
    (Components|Timeline|SetPlayRate _door_track (/ 1.0 (Variables|Default|GetTime%20to%20Open%20%28s%29)))
    (CallFunction|OpenDoor)
    (else
      (Components|Timeline|SetPlayRate _door_track (/ 1.0 (Variables|Default|GetTime%20to%20Open%20%28s%29)))
      (CallFunction|CloseDoor)))
  (return false))