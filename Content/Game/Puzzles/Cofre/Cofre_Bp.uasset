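; A puzzle safe (Cofre) that the player opens with a four-digit code when it is locked.
; InteractSafe opens an unlocked safe directly, or shows the Password widget with the four digits and switches to cursor-driven UI input.
; CheckPassword compares the entry to the joined digits, then on a match calls OpenSafe and restores game input.
; OpenSafe plays a timeline that yaws the door pivot and marks the safe opened.
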(event Custom|OpenSafe
  (bind _alpha (Timeline|SafeOpen PlayFromStart)
    (:Update
      (Variables|SafeAttributes|SetIsLocked? false)
      (Variables|SafeAttributes|SetIsOpened? true)
      (Transformation|SetRelativeRotation (Variables|Default|GetPivot) (Math|Rotator|MakeRotator 0.0 0.0 _alpha) false false))))

(event EventBeginPlay
  (if (not (Variables|SafeAttributes|GetIsOpened?))
    (Transformation|SetRelativeRotation (Variables|Default|GetPivot) "0, 0, 0" false false)))

(event EventInteractSafe
  (bind _returnvalue (Game|GetPlayerController 0))
  (if (not (Variables|SafeAttributes|GetIsOpened?))
    (if (Variables|SafeAttributes|GetIsLocked?)
      (bind _returnvalue_2 (UserInterface|CreateWidget "/Game/Game/Puzzles/Cofre/Password.Password_C" 0 (Variables|GeneratedPassword|GetDigit1) (Variables|GeneratedPassword|GetDigit2) (Variables|GeneratedPassword|GetDigit3) (Variables|GeneratedPassword|GetDigit4) self))
      (bind _output_get (Variables|Default|SetPassword%20UI _returnvalue_2))
      (UserInterface|Viewport|AddtoViewport _output_get 3)
      (Input|SetInputModeUIOnly _returnvalue 0 "DoNotLock" false)
      (Variables|/Script/Engine.PlayerController|SetbShowMouseCursor _returnvalue true)
      (else
        (CallFunction|OpenSafe)))))

(fn ConstructionScript)

(fn CheckPassword
  (bind _returnvalue (Game|GetPlayerController 0))
  (Variables|GeneratedPassword|SetGeneratedPassword "")
  (Variables|GeneratedPassword|SetGeneratedPassword (Utilities|String|Append (Utilities|String|ToString(Integer) (Variables|GeneratedPassword|GetDigit1)) (Utilities|String|ToString(Integer) (Variables|GeneratedPassword|GetDigit2)) (Utilities|String|ToString(Integer) (Variables|GeneratedPassword|GetDigit3)) (Utilities|String|ToString(Integer) (Variables|GeneratedPassword|GetDigit4))))
  (if (Utilities|Enum|Equal(Enum) (Variables|SafeAttributes|GetPassword) (Variables|GeneratedPassword|GetGeneratedPassword))
    (Development|PrintString "Correto")
    (CallFunction|OpenSafe)
    (Widget|RemovefromParent (Variables|Default|GetPassword%20UI))
    (Variables|Default|SetPassword%20UI 0)
    (Input|SetInputModeGameOnly _returnvalue false)
    (Variables|/Script/Engine.PlayerController|SetbShowMouseCursor _returnvalue false)
    (else
      (Development|PrintString "Incorreto"))))

(fn Interact
  (params (Interactor :type Character%20Object%20Reference))
  (return false))