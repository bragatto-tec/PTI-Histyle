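; Door for the figure puzzle that slides open when a SymbolPuzzle actor triggers it.
; OnInteract opens a Gate only if the interacting actor's class is exactly SymbolPuzzle.
; While the gate is open, Tick moves DoorMesh toward the OpenPos relative location at constant speed, with no closing logic.
; The Interact function itself always returns false.
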(event EventOnInteract
  (params (Actor :type Actor%20Object%20Reference) (Hit :type Hit%20Result%20Structure))
  (if (== (Utilities|GetClass Actor) "/Game/Game/Puzzles/figurepuzzle/SymbolPuzzle.SymbolPuzzle_C")
    (Utilities|FlowControl|Gate true) ; enters at Open
  ))

(event EventTick
  (params (DeltaSeconds :type Float%20%28single-precision%29))
  (Utilities|FlowControl|Gate true
    (:Exit
      (Transformation|SetRelativeLocation (Variables|Default|GetDoor%20Mesh) (Math|Interpolation|VInterptoConstant (Variables|/Script/Engine.SceneComponent|GetRelativeLocation (Variables|Default|GetDoor%20Mesh)) (Variables|/Script/Engine.SceneComponent|GetRelativeLocation (Variables|Default|GetOpen_Pos)) DeltaSeconds 1e+02) false false))))

(fn ConstructionScript)

(fn Interact
  (params (Interactor :type Character%20Object%20Reference))
  (return false))