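; Zombie enemy that chases the player through a self-repeating AIMoveTo on the player controller, changing walk speed when PawnSensing sees a pawn.
; Capsule overlap plays an attack montage, whose notify applies damage through a sphere check at Arrow1.
; Montage completion resumes the chase and also calls DamagePlayer on the overlapped character.
; Point damage reduces Health, playing a hit reaction or a death montage followed by delayed destruction.
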(event OnComponentBeginOverlap(CapsuleComponent)
  (params (OverlappedComponent :type Primitive%20Component%20Object%20Reference) (OtherActor :type Actor%20Object%20Reference) (OtherComp :type Primitive%20Component%20Object%20Reference) (OtherBodyIndex :type Integer) (bFromSweep :type Boolean) (SweepResult :type Hit%20Result%20Structure%20%28by%20ref%29))
  (CallFunction|AttackPlayer))

(event OnSeePawn(PawnSensing)
  (params (Pawn :type Pawn%20Object%20Reference))
  (Variables|/Script/Engine.CharacterMovementComponent|SetMaxWalkSpeed (Variables|Character|GetCharacterMovement) 3.6e+02))

(event Custom|Death
  (Variables|Default|SetIsDead? true)
  (if true
    (Components|Movement|StopMovementImmediately (Variables|Character|GetCharacterMovement))
    (Animation|Montage|PlayMontage (Variables|Character|GetMesh) "/Game/Inimigos/Animations/zombie_dying_Montage1.zombie_dying_Montage1"
      (:then
        (Utilities|FlowControl|Delay 5.0)
        (Actor|DestroyActor)))
    (else
      (Audio|Components|Audio|Stop (Variables|Character|GetMesh)))))

(event Custom|RunToPlayer
  (if (not (Variables|Default|GetIsDead?))
    (AI|AIMoveTo self "0, 0, 0" (Game|GetPlayerController 0) 4e+01 false
      (:OnSuccess
        _)
      (:OnFail
        _))
    (CallFunction|RuntoPlayer)))

(event Custom|AttackPlayer
  ;[1 1 1] ATACAR JOGADOR
  (Animation|Montage|PlayMontage (Variables|Character|GetMesh) "/Game/Inimigos/Animations/zombie_attack_Montage1.zombie_attack_Montage1"
    (:OnCompleted
      (CallFunction|RuntoPlayer)
      (bind _asbp_first_person_character (Utilities|Casting|CastToBP_FirstPersonCharacter (stale OnComponentBeginOverlap(CapsuleComponent) OtherActor)))
      (Default|DamagePlayer _asbp_first_person_character))
    (:OnNotifyBegin
      (bind (_outactors _returnvalue) (Collision|SphereOverlapActors (Transformation|GetWorldLocation (Variables|Default|GetArrow1)) 8e+01 (Utilities|Array|MakeArray "ObjectTypeQuery3") "/Game/FirstPerson/Blueprints/BP_FirstPersonCharacter.BP_FirstPersonCharacter_C" (Utilities|Array|MakeArray self)))
      (if _returnvalue
        (for _array_element _outactors
          (Game|Damage|ApplyDamage _array_element 2e+01 (Pawn|GetController) self "/Script/Engine.DamageType"))))))

(event EventBeginPlay
  (CallFunction|RuntoPlayer))

(event Game|Damage|EventPointDamage
  (params (Damage :type Float%20%28single-precision%29) (DamageType :type Damage%20Type%20Object%20Reference) (HitLocation :type Vector :default "0, 0, 0") (HitNormal :type Vector :default "0, 0, 0") (HitComponent :type Primitive%20Component%20Object%20Reference) (BoneName :type Name :default "None") (ShotFromDirection :type Vector :default "0, 0, 0") (InstigatedBy :type Controller%20Object%20Reference) (DamageCauser :type Actor%20Object%20Reference) (HitInfo :type Hit%20Result%20Structure%20%28by%20ref%29))
  (if (not (Variables|Default|GetIsDead?))
    (if (<= (Variables|Default|GetHealth) 0.0)
      (CallFunction|Death)
      (else
        (bind _output_get (Variables|Default|SetHealth (- (Variables|Default|GetHealth) Damage)))
        (Development|PrintString (Utilities|String|ToString(Float) _output_get))
        (if (<= _output_get 0.0)
          (CallFunction|Death)
          (else
            (Animation|Montage|PlayMontage (Variables|Character|GetMesh) "/Game/Inimigos/Animations/Zombie_Reaction_Hit_Anim_mixamo_com_Montage.Zombie_Reaction_Hit_Anim_mixamo_com_Montage")))))))

(fn ConstructionScript)